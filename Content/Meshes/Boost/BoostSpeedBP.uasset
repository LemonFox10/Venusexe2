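; Speed boost pickup that temporarily doubles a FirstPersonCharacter's max walk speed when it overlaps the Shoes component.
; A timeline acts as the boost timer, restoring normal speed when finished and printing the speed at each change.
; After a short delay the actor destroys itself and calls ReSpawn, which spawns an actor at one of the first three TargetPoint_Blueprint actors, picked at random.
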(event OnComponentBeginOverlap(Shoes)
  (params (OverlappedComponent :type Primitive%20Component%20Object%20Reference) (OtherActor :type Actor%20Object%20Reference) (OtherComp :type Primitive%20Component%20Object%20Reference) (OtherBodyIndex :type Integer) (bFromSweep :type Boolean) (SweepResult :type Hit%20Result%20Structure%20%28by%20ref%29))
  (bind _asfirst_person_character (Utilities|Casting|CastToFirstPersonCharacter OtherActor))
  (Variables|/Script/Engine.CharacterMovementComponent|SetMaxWalkSpeed (Variables|/Script/Engine.Character|GetCharacterMovement _asfirst_person_character) 1.4e+03)
  (Development|PrintString (Utilities|String|ToString(Float) (Class|MovementComponent|GetMaxSpeed (Variables|/Script/Engine.Character|GetCharacterMovement _asfirst_person_character))))
  (Timeline|Línea%20de%20tiempo_0 PlayFromStart
    (:Finished
      (Variables|/Script/Engine.CharacterMovementComponent|SetMaxWalkSpeed (Variables|/Script/Engine.Character|GetCharacterMovement _asfirst_person_character) 7e+02)
      (Development|PrintString (Utilities|String|ToString(Float) (Class|MovementComponent|GetMaxSpeed (Variables|/Script/Engine.Character|GetCharacterMovement _asfirst_person_character))))
      (Utilities|FlowControl|Delay 0.2)
      (Actor|DestroyActor)
      (CallFunction|ReSpawn))))

(event Custom|ReSpawn
  (bind _outactors (Actor|GetAllActorsOfClass "/Game/FirstPersonBP/Blueprints/TargetPoint_Blueprint.TargetPoint_Blueprint_C"))
  (Game|SpawnActorfromClass "BoostSpeedBP_C" (Transformation|GetActorTransform (Utilities|Array|Get(acopy) _outactors (Math|Random|RandomIntegerinRange 0 2))) "AdjustIfPossibleButAlwaysSpawn" 0 0))

(fn ConstructionScript)